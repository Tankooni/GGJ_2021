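; HexTile is a hex tile Blueprint whose color and height can be changed at runtime.
; BeginPlay creates a dynamic material instance for the tile and prints its current height.
; SetColor writes a random RGB value to that instance's Color parameter.
; SetHeight increments Height, wrapping to 1 once it exceeds five, and applies it as the world Z scale.
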(event EventBeginPlay
  (bind _returnvalue (Rendering|Material|CreateDynamicMaterialInstance 0 0 "None" :!class /Script/Engine.PrimitiveComponent))
  (Variables|Default|SetMaterialInstance _returnvalue)
  (Development|PrintString (Utilities|String|ToString(Integer) (Variables|Default|GetHeight))))

(fn SetColor
  (Rendering|Material|SetVectorParameterValue (Variables|Default|GetMaterialInstance) "Color" (Utilities|Struct|MakeLinearColor (Math|Random|RandomFloat) (Math|Random|RandomFloat) (Math|Random|RandomFloat) 1.0) :!class /Script/Engine.MaterialInstanceDynamic))

(fn SetHeight
  (if (> (Variables|Default|GetHeight) 5)
    (Variables|Default|SetHeight 1)
    (else
      (Math|Integer|IncrementInt (Variables|Default|GetHeight)
        (:%20%20
          _))))
  (Transformation|SetWorldScale3D (Math|Vector|MakeVector 1.0 1.0 (Math|Conversions|ToFloat(Integer) (Variables|Default|GetHeight)))))